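; Gameplay ability for the player's primary attack, alternating between two montages (A and B) through a FlipFlop.
; The ability ends when the montage completes, blends out or is interrupted or cancelled.
; In parallel, it waits for the Primary gameplay event, then runs a hitbox overlap test and sends hit react events to the actors found.
; A debug sphere drawing of the hitbox is present but unconnected.
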(event Ability|EventActivateAbility
  (Utilities|FlowControl|Sequence
    (:then_0
      ;[0.000254 0.02238 0.15 0.5] Play Attack Montage
      (Utilities|FlowControl|FlipFlop
        (:A
          (|PlayMontageandWaitProxy "None" "/Game/crashcourse/Characters/PlayerCharacter/Animations/CC_Primary_A_Montage.CC_Primary_A_Montage" 1.0 "None" true 1.0 0.0 false
            (:OnCompleted
              _)
            (:OnBlendOut
              _)
            (:OnInterrupted
              _)
            (:OnCancelled
              _))
          (Ability|EndAbility))
        (:B
          (|PlayMontageandWaitProxy "None" "/Game/crashcourse/Characters/PlayerCharacter/Animations/CC_Primary_B_Montage.CC_Primary_B_Montage" 1.0 "None" true 1.0 0.0 false
            (:OnCompleted
              _)
            (:OnBlendOut
              _)
            (:OnInterrupted
              _)
            (:OnCancelled
              _))
          (Ability|EndAbility))))
    (:then_1
      (Ability|Tasks|WaitGameplayEvent "(TagName=\"CCTags.Events.Player.Primary\")" 0
        (:EventReceived
          (bind _returnvalue (Class|CCPrimary|HitBoxOverlapTest))
          (Class|CCPrimary|SendHitReactEventtoActors _returnvalue))))))

(event Ability|EventOnEndAbility
  (params (bWasCancelled :type Boolean)))