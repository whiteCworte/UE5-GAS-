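; Enemy gameplay ability that plays a directional hit reaction montage in response to the HitReact gameplay event.
; On activation it waits for the event, then caches direction vectors from the payload's instigator and derives a hit direction name from them.
; It plays the montage and jumps to the section with that name, with optional debug prints.
; The graph never ends the ability.
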(event Ability|EventActivateAbility
  (bind _payload (Ability|Tasks|WaitGameplayEvent "(TagName=\"CCTags.Events.Enemy.HitReact\")" 0)
    (:EventReceived
      (CallFunction|PrintDebugEventReceived _payload)
      (Class|CCHitReact|CacheHitDirectionVectors (.Instigator (Utilities|Struct|BreakGameplayEventData _payload)))
      (Utilities|FlowControl|Sequence
        (:then_0
          ;[0.02285 0.005441 0.15 0.5] Cache Hit Direction Name
          (Variables|Default|SetHitDirectionName (Class|CCBlueprintLibrary|GetHitDirectionName (Class|CCBlueprintLibrary|GetHitDirection (Variables|Default|GetAvatorForward) (Variables|Default|GetToInstigator))))
          ;[0.5043 0 0.01525 0.5] Debug for Hit Direction
          (Variables|Default|GetbDrawDebugs
            (:then
              (Development|PrintString (Utilities|String|ToString(Name) (Variables|Default|GetHitDirectionName))))
            (:else)))
        (:then_1
          (|PlayMontageandWaitProxy "None" (Variables|Default|GetHitReactMontage) 1.0 "None" true 1.0 0.0 false
            (:then
              (Ability|Animation|MontageJumptoSection (Variables|Default|GetHitDirectionName)))))))))

(event Ability|EventOnEndAbility
  (params (bWasCancelled :type Boolean)))

(fn PrintDebugEventReceived
  (params (GameplayEventData :type Gameplay%20Event%20Data%20Structure%20%28by%20ref%29))
  (Variables|Default|GetbDrawDebugs
    (:then
      (Development|PrintString (Utilities|String|Append (Utilities|GetDisplayName (.Instigator (Utilities|Struct|BreakGameplayEventData GameplayEventData))) "") true true "(R=1.000000,G=0.000000,B=0.782623,A=1.000000)"))
    (:else)))